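; Weapon actor that, on WeaponFire, plays firing effects and spawns a projectile from its starting point.
; Firing triggers particle and sound, with a timer to deactivate the flash and spotlight, although only BeginPlay and that timer touch their activation.
; Spawned OMockExtendedProjectiles receive the parent actor's tags as collision-dismiss tags, then get activated.
; FXColoursEdit applies a custom colour to both lights.
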(event `WeaponFire`
  ;[1 1 1] Weapon Fire
  (`self.ActivateFXs`)
  (`self.SpawnProjectile`))

(event `ActivateFXs`
  ;[1 1 1] FX Activation
  (`KismetSystemLibrary.K2_SetTimerDelegate` (delegate `DeactivateFXs`) (`self.FXDeactivationTimeSeconds`))
  (`ActorComponent.Activate` (`self.WeaponFiringParticle`) true)
  (`AudioComponent.Play` (`self.WeaponFiringSoundCue`) 0.0))

(event `DeactivateFXs`
  ;[1 1 1] FX Deactivation
  (`ActorComponent.Deactivate` (`self.WeaponFiringFlash`))
  (`ActorComponent.Deactivate` (`self.WeaponFiringSpotlight`)))

(event `SpawnProjectile`
  (bind _returnvalue (`SceneComponent.K2_GetComponentToWorld` (`self.ProjectileStartingPoint`)))
  ;[1 1 1] Projectile Spawning
  ;;[1 1 1] Spawn Actor
  (bind _returnvalue_2 (`|SpawnActorFromClass` (`self.ProjectileClassTemplate`) _returnvalue "AdjustIfPossibleButAlwaysSpawn" "OverrideRootScale" null _returnvalue))
  ;;[1 1 1] Additional Spawn Event
  (bind _asomock_extended_projectile (cast `/Game/Scripts/Blueprints/Projectiles/OMockExtendedProjectile` _returnvalue_2)
    (:`then`
      (message `/Game/Scripts/Blueprints/Projectiles/IProjectile.Spawn` _asomock_extended_projectile _returnvalue (`Actor.Tags` (`self.GetParentActor`)) null)
      ;;[1 1 1] Activating
      (message `/Game/Scripts/Blueprints/Projectiles/IProjectile.Activate` _asomock_extended_projectile)
      (`/Game/Scripts/Blueprints/Projectiles/OBaseProjectile.Activate` _asomock_extended_projectile))
    (:`CastFailed`
      (message `/Game/Scripts/Blueprints/Projectiles/IProjectile.Deactivate` _asomock_extended_projectile))))

(event `self.ReceiveBeginPlay`
  ;[1 1 1] Deactivate FXs (onStart)
  ;;[1 1 1] WeaponFlash
  (`ActorComponent.Deactivate` (`self.WeaponFiringFlash`))
  ;;[1 1 1] Sound Cue
  (`ActorComponent.Deactivate` (`self.WeaponFiringSoundCue`))
  ;;[1 1 1] Particle
  (`ActorComponent.Deactivate` (`self.WeaponFiringParticle`))
  ;;[1 1 1] Spotlight
  (`ActorComponent.Deactivate` (`self.WeaponFiringSpotlight`)))

(fn `FXColoursEdit`
  (params (WeaponFXsColour :type "LinearColor Structure"))
  (bind _output_get (set `self.WeaponFXsColour` WeaponFXsColour))
  (set `self.isCustomFXColourUsed` true)
  (`LightComponent.SetLightColor` (`self.WeaponFiringSpotlight`) _output_get true)
  (`LightComponent.SetLightColor` (`self.WeaponFiringFlash`) _output_get true))

(fn `UserConstructionScript`)