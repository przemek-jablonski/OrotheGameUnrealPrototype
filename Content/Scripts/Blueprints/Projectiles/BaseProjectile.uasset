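; Base projectile actor that damages what it hits and dies on impact or when its lifetime timer runs out.
; Spawn stores setup data, fires an empty spawn-FX hook and starts the Kill timer.
; HandleCollision skips actors matching dismiss or own tags, damages IDamageable ones and calls Kill, while any actor overlap kills directly.
; Kill waits a frame, spawns the death-FX actor and destroys itself; Activate/Deactivate toggle movement and body child components.
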(event `/Game/Scripts/Blueprints/Projectiles/IProjectile.Activate`
  ;[1 1 1] Component Activation
  (for _array_element (`SceneComponent.GetChildrenComponents` (`self.ProjectileBodySM`) true)
    (`ActorComponent.Activate` _array_element false))
  (`ActorComponent.Activate` (`self.ProjectileMovement`) false))

(event `SetVariables`
  ;[1 1 1] Setting Variables
  (set `self.collisionDismissTags` (stale `/Game/Scripts/Blueprints/Projectiles/IProjectile.Spawn` collisionDismissTags))
  (set `self.projectileDeathFxClassTemplate` (stale `/Game/Scripts/Blueprints/Projectiles/IProjectile.Spawn` projectileDeathFxClassTemplate)))

(event `/Game/Scripts/Blueprints/Projectiles/IProjectile.Deactivate`
  ;[1 1 1] Component Deactivation
  (for _array_element (`SceneComponent.GetChildrenComponents` (`self.ProjectileBodySM`) true)
    (`ActorComponent.Deactivate` _array_element))
  (`ActorComponent.Deactivate` (`self.ProjectileMovement`)))

(event `/Game/Scripts/Blueprints/Projectiles/IProjectile.Spawn`
  (params (spawnPositionTransform :type "Transform Structure") (collisionDismissTags :type "Array of Name (by ref)") (projectileDeathFxClassTemplate :type "Actor Class Reference"))
  ;[1 1 1] Handling Spawn Event
  (`self.SetVariables`)
  (`self.ActivateSpawnFX` spawnPositionTransform)
  (`KismetSystemLibrary.K2_SetTimerDelegate` (delegate `Kill`) (`self.projectileDestroyTime`)))

(event `Kill`
  ;[1 1 1] Handling Kill Event
  (`KismetSystemLibrary.Delay` (`GameplayStatics.GetWorldDeltaSeconds`))
  (`self.ActivateDeathFX` (`SceneComponent.K2_GetComponentToWorld` (`self.CollisionMesh`)))
  (`self.K2_DestroyActor`))

(event `/Game/Scripts/Blueprints/Projectiles/IProjectile.ActivateSpawnFX`
  (params (spawnPositionTransformParam :type "Transform Structure")))

(event `/Game/Scripts/Blueprints/Projectiles/IProjectile.ActivateDeathFX`
  (params (deathPositionTransform :type "Transform Structure"))
  (`|SpawnActorFromClass` (`self.projectileDeathFxClassTemplate`) deathPositionTransform "AdjustIfPossibleButAlwaysSpawn" "OverrideRootScale"))

(event `/Game/Scripts/Blueprints/Projectiles/IProjectile.HandleCollision`
  (params (collidedActor :type "Actor Object Reference"))
  (bind _hascollisiondismisstag (`self.hasCollisionTag` collidedActor (`self.collisionDismissTags`)))
  (if (not _hascollisiondismisstag)
    (bind _hascollisiondismisstag_2 (`self.hasCollisionTag` collidedActor (`self.Tags`)))
    (if (not _hascollisiondismisstag_2)
      (if (`KismetSystemLibrary.DoesImplementInterface` collidedActor "/Game/Scripts/Blueprints/Interfaces/IDamageable.IDamageable_C")
        (message `/Game/Scripts/Blueprints/Interfaces/IDamageable.DealDamage` collidedActor (`self.damageData`)))
      (`self.Kill`))))

(event `self.ReceiveActorBeginOverlap`
  (params (OtherActor :type "Actor Object Reference"))
  (`self.Kill`))

(fn `hasCollisionTag`
  (params (actor :type "Actor Object Reference") (checkingCollisions :type "Array of Name"))
  (returns (hasCollisionDismissTag :type Boolean))
  (locals (collisionDismissTagOccured :type Boolean :default false))
  (bind _collisiondismisstagoccured (`local.collisionDismissTagOccured`))
  (for _array_element checkingCollisions
    (if (`self.ActorHasTag` actor _array_element)
      (set `local.collisionDismissTagOccured` true)
      (return _collisiondismisstagoccured)))
  (return _collisiondismisstagoccured))

(fn `UserConstructionScript`)