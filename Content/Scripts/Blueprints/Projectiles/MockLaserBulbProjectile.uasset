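; Laser bulb projectile actor that deals fixed damage to IDamageable actors and self-destructs on a lifetime timer set at BeginPlay.
; Damage fires when an overlap ends, skipping actors with the parent's first tag or the dismiss tag, then destruction follows a brief delay.
; Destruction removes body and movement and plays death particles, whose completion destroys the actor.
; An optional custom colour is applied through a dynamic material instance at spawn.
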(event `SpawnProjectile`
  (bind _projectilebody (`self.ProjectileBody`))
  ;[1 1 1] Projectile Spawning
  (`KismetSystemLibrary.K2_SetTimerDelegate` (delegate `DestroyProjectile`) (`self.ProjectileDeathTimerSec`))
  ;;[1 1 1] ChangingColour
  (if (`self.isCustomFXColourUsed`)
    (bind _returnvalue (`PrimitiveComponent.CreateDynamicMaterialInstance` _projectilebody 0 (`PrimitiveComponent.GetMaterial` _projectilebody 0)))
    (`KismetMaterialLibrary.SetVectorParameterValue` null (`self.LaserColorName`) (`self.ProjectileFXColour`))
    (`PrimitiveComponent.SetMaterial` _projectilebody 0 _returnvalue)))

(event `DestroyProjectile`
  ;[1 1 1] Destroying Projectile
  ;;[1 1 1] Checking Pending Kill event
  (if (not (`self.isPendingKill`))
    (set `self.isPendingKill` true)
    ;;[1 1 1] Activating Death FX
    (`ActorComponent.Activate` (`self.ParticleSystemDeath`) false)
    ;;[1 1 1] Destroying other Components
    (`ActorComponent.K2_DestroyComponent` (`self.ProjectileBody`))
    (`ActorComponent.K2_DestroyComponent` (`self.ProjectileMovement`))))

(event `self.ParticleSystemDeath.OnParticleDeath`
  (params (EventName :type Name) (EmitterTime :type "Float (single-precision)") (ParticleTime :type Integer) (Location :type "Vector Structure") (Velocity :type "Vector Structure") (Direction :type "Vector Structure"))
  ;[1 1 1] Destroying Projectile
  ;;[1 1 1] onDeathParticleFinished
  (`self.onDestroy` :!label _label)
  (`self.K2_DestroyActor`))

(event `self.ParticleSystemDeath.OnSystemFinished`
  (params (PSystem :type "ParticleSystemComponent Object Reference"))
  ;[1 1 1] Destroying Projectile
  ;;[1 1 1] onDeathParticleFinished
  (goto _label))

(event `self.ReceiveBeginPlay`
  ;[1 1 1] Constructing
  (`self.SpawnProjectile`))

(event `self.ReceiveActorEndOverlap`
  (params (OtherActor :type "Actor Object Reference"))
  ;[1 1 1] Collisions
  (if (`self.ActorHasTag` OtherActor (`KismetArrayLibrary.Array_Get` (`self.parentActorTags`)))
    _
    (elif (not (`self.ActorHasTag` OtherActor (`self.ProjectileCollisionDismissTag`)))
      (if (`KismetSystemLibrary.DoesImplementInterface` OtherActor "/Game/Scripts/Blueprints/Interfaces/IDamageable.IDamageable_C")
        (message `/Game/Scripts/Blueprints/Interfaces/IDamageable.DealDamage` OtherActor (`|MakeArray` (make `/Game/Scripts/Blueprints/DataStructures/OSProjectileDamageStruct` "NewEnumerator0" 35.0))))
      (`KismetSystemLibrary.Delay` (* (`GameplayStatics.GetWorldDeltaSeconds`) 2.0))
      (`self.DestroyProjectile`))))

(event `Activate`
  ;[1 1 1] Activate
  (`ActorComponent.Activate` (`self.DefaultSceneRoot`) false)
  (`ActorComponent.Activate` (`self.ProjectileMovement`) false))

(event `Deactivate`
  ;[1 1 1] Deactivate
  (`ActorComponent.Deactivate` (`self.DefaultSceneRoot`))
  (`ActorComponent.Deactivate` (`self.ProjectileMovement`)))

(fn `Construct`
  (params (parentActorTags :type "Array of Name"))
  (set `self.parentActorTags` parentActorTags))

(fn `onDestroy`
  (returns (Position :type "Vector Structure") (Rotation :type "Rotator Structure"))
  (return (0.0 0.0 0.0)))

(fn `SetProjectileFXColour`
  (params (ProjectileFXColour :type "LinearColor Structure"))
  (set `self.ProjectileFXColour` ProjectileFXColour)
  (set `self.isCustomFXColourUsed` true))

(fn `UserConstructionScript`)