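; Laser bulb projectile actor that self-destructs after a lifetime timer set on BeginPlay or shortly after it stops overlapping another actor.
; End overlaps ignore actors tagged as player, player weapon or projectile; others trigger destruction after a two-frame delay.
; A guarded DestroyProjectile activates death particles and removes body and movement components.
; Particle death or completion calls OnDestroy, which returns only zero transform values, then destroys the actor.
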(event `self.ReceiveActorEndOverlap`
  (params (OtherActor :type "Actor Object Reference"))
  (if (not (or (`self.ActorHasTag` OtherActor (`self.PlayerActorCollisionDismissTag`)) (`self.ActorHasTag` OtherActor (`self.PlayerWeaponCollisionDismissTag`)) (`self.ActorHasTag` OtherActor (`self.ProjectileCollisionDismissTag`))))
    (`KismetSystemLibrary.Delay` (* (`GameplayStatics.GetWorldDeltaSeconds`) 2.0))
    (`self.DestroyProjectile`)))

(event `SpawnProjectile`
  ;[1 1 1] Projectile Spawning
  (`KismetSystemLibrary.K2_SetTimerDelegate` (delegate `DestroyProjectile`) (`self.ProjectileDeathTimerSec`)))

(event `DestroyProjectile`
  ;[1 1 1] Destroying Projectile
  ;;[1 1 1] Checking Pending Kill event
  (if (not (`self.isPendingKill`))
    (set `self.isPendingKill` true)
    ;;[1 1 1] Activating Death FX
    (`ActorComponent.Activate` (`self.ParticleSystemDeath`) false)
    ;;[1 1 1] Destroying other Components
    (`ActorComponent.K2_DestroyComponent` (`self.ProjectileBody`))
    (`ActorComponent.K2_DestroyComponent` (`self.ProjectileMovement`))))

(event `self.ParticleSystemDeath.OnParticleDeath`
  (params (EventName :type Name) (EmitterTime :type "Float (single-precision)") (ParticleTime :type Integer) (Location :type "Vector Structure") (Velocity :type "Vector Structure") (Direction :type "Vector Structure"))
  ;[1 1 1] Destroying Projectile
  ;;[1 1 1] onDeathParticleFinished
  (`self.onDestroy` :!label _label)
  (`self.K2_DestroyActor`))

(event `self.ParticleSystemDeath.OnSystemFinished`
  (params (PSystem :type "ParticleSystemComponent Object Reference"))
  ;[1 1 1] Destroying Projectile
  ;;[1 1 1] onDeathParticleFinished
  (goto _label))

(event `self.ReceiveBeginPlay`
  ;[1 1 1] Constructing
  (`self.SpawnProjectile`))

(fn `onDestroy`
  (returns (Position :type "Vector Structure") (Rotation :type "Rotator Structure"))
  (return (0.0 0.0 0.0)))

(fn `UserConstructionScript`)