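; Player character Blueprint for an over-the-shoulder style shooter, handling movement, sprinting, look, aiming and firing.
; Movement follows control yaw scaled by a jog or sprint multiplier, while vertical look also rotates the MockWeapon child actor component.
; Aiming instantly switches spring arm length and socket offset, using an aim length derived at BeginPlay.
; Firing calls WeaponFire on the first world actor of the weapon's class, rather than the component's own child.
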(event `InputAxis|MovementVertical`
  (params (AxisValue :type "Float (single-precision)"))
  (bind (_returnvalue_roll _returnvalue_pitch _returnvalue_yaw) (`KismetMathLibrary.BreakRotator` (`self.GetControlRotation`)))
  ;[1 1 1] Movement
  (`self.AddMovementInput` (`KismetMathLibrary.GetForwardVector` (`KismetMathLibrary.MakeRotator` 0.0 0.0 _returnvalue_yaw)) (* AxisValue (stale `InputAction|Sprint` _output_get))))

(event `InputAxis|MovementHorizontal`
  (params (AxisValue :type "Float (single-precision)"))
  (bind (_returnvalue_roll _returnvalue_pitch _returnvalue_yaw) (`KismetMathLibrary.BreakRotator` (`self.GetControlRotation`)))
  ;[1 1 1] Movement
  (`self.AddMovementInput` (`KismetMathLibrary.GetRightVector` (`KismetMathLibrary.MakeRotator` 0.0 0.0 _returnvalue_yaw)) (* AxisValue (stale `InputAction|Sprint` _output_get))))

(event `InputAction|Sprint`
  (params (Key :type "Key Structure" :default "AnyKey"))
  ;[1 1 1] Movement
  ;;[1 1 1] Sprinting multiplier
  (:`Pressed`
    (set `self.SprintPressed` true)
    (bind _output_get (set `self.CurrentSpeedMultiplier` (`self.SprintMultiplier`))))
  (:`Released`
    (set `self.SprintPressed` false)
    (bind _output_get_2 (set `self.CurrentSpeedMultiplier` (`self.JogMultiplier`)))))

(event `InputAxis|RotationVertical`
  (params (AxisValue :type "Float (single-precision)"))
  (bind _returnvalue (`GameplayStatics.GetWorldDeltaSeconds`))
  (bind _baseturn (`self.BaseTurn`))
  ;[1 1 1] Rotation
  (`self.AddControllerPitchInput` (* AxisValue _baseturn _returnvalue))
  (`SceneComponent.K2_AddLocalRotation` (`self.MockWeapon`) (`KismetMathLibrary.MakeRotator` (* AxisValue _returnvalue _baseturn)) false false))

(event `InputAxis|RotationHorizontal`
  (params (AxisValue :type "Float (single-precision)"))
  ;[1 1 1] Rotation
  (`self.AddControllerYawInput` (* (`self.BaseTurn`) (`GameplayStatics.GetWorldDeltaSeconds`) AxisValue)))

(event `ConstructVariables`
  ;[1 1 1] ConstructVariables
  ;;[1 1 1] Starting Movement Speed
  (set `self.CurrentSpeedMultiplier` (`self.JogMultiplier`))
  ;;[1 1 1] Cam Arm Length (normal)
  (set `self.CamNormalArmLength` (`SpringArmComponent.TargetArmLength` (`self.SpringArm`)))
  (set `SpringArmComponent.TargetArmLength` (`self.CamNormalArmLength`) (`self.SpringArm`))
  ;;[1 1 1] Cam Arm Length (aiming)
  (set `self.CamAimingArmLengthDiv` (/ (`self.CamNormalArmLength`) (`self.CamAimingArmLengthDiv`))))

(event `self.ReceiveBeginPlay`
  ;[1 1 1] Setting variables
  (`self.ConstructVariables`))

(event `InputAction|Aim`
  (params (Key :type "Key Structure" :default "AnyKey"))
  (bind _springarm (`self.SpringArm`))
  ;[1 1 1] Aiming
  (:`Pressed`
    (set `SpringArmComponent.TargetArmLength` (`self.CamAimingArmLengthDiv`) _springarm)
    (set `SpringArmComponent.SocketOffset` (`self.CamAimingArmOffset`) _springarm))
  (:`Released`
    (set `SpringArmComponent.TargetArmLength` (`self.CamNormalArmLength`) _springarm)
    (set `SpringArmComponent.SocketOffset` (0.0 0.0 100.0) _springarm)))

(event `InputAction|Fire`
  (params (Key :type "Key Structure" :default "AnyKey"))
  ;[1 1 1] Firing
  (:`Pressed`
    (bind _outactors (`GameplayStatics.GetAllActorsOfClass` (`ChildActorComponent.ChildActorClass` (`self.MockWeapon`))))
    (bind _asmock_weapon (cast `/Game/Scripts/Blueprints/Weaponry/MockWeapon` (`KismetArrayLibrary.Array_Get` _outactors)))
    (`/Game/Scripts/Blueprints/Weaponry/MockWeapon.WeaponFire` _asmock_weapon)))

(fn `UserConstructionScript`)