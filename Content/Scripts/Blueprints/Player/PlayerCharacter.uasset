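; Player character Blueprint that handles movement, sprinting and camera rotation input.
; Movement axes add input along control-yaw forward and right vectors, scaled by CurrentSpeedMultiplier.
; Sprint switches that multiplier between jog, the BeginPlay default, and sprint values, changing input scale rather than movement component speed.
; Rotation axes feed controller pitch and yaw, scaled by BaseTurn and frame delta time.
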(event `InputAxis|MovementVertical`
  (params (AxisValue :type "Float (single-precision)"))
  (bind (_returnvalue_roll _returnvalue_pitch _returnvalue_yaw) (`KismetMathLibrary.BreakRotator` (`self.GetControlRotation`)))
  ;[1 1 1] Movement
  (`self.AddMovementInput` (`KismetMathLibrary.GetForwardVector` (`KismetMathLibrary.MakeRotator` 0.0 0.0 _returnvalue_yaw)) (* AxisValue (stale `InputAction|Sprint` _output_get))))

(event `InputAxis|MovementHorizontal`
  (params (AxisValue :type "Float (single-precision)"))
  (bind (_returnvalue_roll _returnvalue_pitch _returnvalue_yaw) (`KismetMathLibrary.BreakRotator` (`self.GetControlRotation`)))
  ;[1 1 1] Movement
  (`self.AddMovementInput` (`KismetMathLibrary.GetRightVector` (`KismetMathLibrary.MakeRotator` 0.0 0.0 _returnvalue_yaw)) (* AxisValue (stale `InputAction|Sprint` _output_get))))

(event `InputAction|Sprint`
  (params (Key :type "Key Structure" :default "AnyKey"))
  ;[1 1 1] Movement
  ;;[1 1 1] Sprinting multiplier
  (:`Pressed`
    (set `self.SprintPressed` true)
    (bind _output_get (set `self.CurrentSpeedMultiplier` (`self.SprintMultiplier`))))
  (:`Released`
    (set `self.SprintPressed` false)
    (bind _output_get_2 (set `self.CurrentSpeedMultiplier` (`self.JogMultiplier`)))))

(event `InputAxis|RotationVertical`
  (params (AxisValue :type "Float (single-precision)"))
  ;[1 1 1] Rotation
  (`self.AddControllerPitchInput` (* AxisValue (`self.BaseTurn`) (`GameplayStatics.GetWorldDeltaSeconds`))))

(event `InputAxis|RotationHorizontal`
  (params (AxisValue :type "Float (single-precision)"))
  ;[1 1 1] Rotation
  (`self.AddControllerYawInput` (* (`self.BaseTurn`) (`GameplayStatics.GetWorldDeltaSeconds`) AxisValue)))

(event `self.ReceiveBeginPlay`
  (set `self.CurrentSpeedMultiplier` (`self.JogMultiplier`)))

(fn `UserConstructionScript`)