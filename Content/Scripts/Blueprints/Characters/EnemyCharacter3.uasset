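; Enemy character with a randomized body colour, health and a weapon held as a MockWeapon child actor.
; BeginPlay sets jog speed and a random shooting-distance threshold, then randomizes appearance, as does the construction script, through a dynamic material instance and red weapon FX tint.
; DealDamage subtracts each damage entry from health, spawning fire FX and destroying the actor below zero.
; WeaponFire forwards firing to the weapon.
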(event `self.ReceiveBeginPlay`
  ;[1 1 1] Begin Play
  (`self.ConstructVariables`)
  (`self.RandomizeAppearance`))

(event `ConstructVariables`
  ;[1 1 1] Construct
  (`|ExecutionSequence`
    (:`then_0`
      ;;[1 1 1] Starting Movement Speed
      (set `self.CurrentSpeedMultiplier` (`self.JogMultiplier`))
      ;;[1 1 1] Shooting Distance
      (set `self.EnemyShootingDistanceThreshold` (+ (`KismetMathLibrary.RandomFloatInRange` 0.0 2000.0) (`self.EnemyShootingDistanceMin`))))))

(event `/Game/Scripts/Blueprints/Interfaces/IDamageable.DealDamage`
  (params (damageData :type "Array of /Game/Scripts/Blueprints/DataStructures/OSProjectileDamageStruct Structure (by ref)"))
  (bind (_returnvalue_location _returnvalue_rotation _returnvalue_scale) (`KismetMathLibrary.BreakTransform` (`self.GetTransform`)))
  ;[1 1 1] Damaged
  (for _array_element damageData
    (bind _output_get (set `self.healthPoints` (- (`self.healthPoints`) (`.damageTypeValue_5_E91F56ED41F15A2D7E6080955AB4F4A6` (break `/Game/Scripts/Blueprints/DataStructures/OSProjectileDamageStruct` _array_element)))))
    (`KismetSystemLibrary.PrintString` (`KismetStringLibrary.BuildString_Double` "ENEMY HP: " "" _output_get))
    (if (< _output_get 0.0)
      (`|SpawnActorFromClass` "/Game/Scripts/Blueprints/FXs/FireFX.FireFX_C" (`KismetMathLibrary.MakeTransform` (- _returnvalue_location (0.0 120.0 0.0)) _returnvalue_rotation _returnvalue_scale) "Undefined" "OverrideRootScale")
      (`self.K2_DestroyActor`))))

(event `RandomizeAppearance`
  (bind _mesh (`self.Mesh`))
  ;[1 1 1] Randomize Appearance
  ;;[1 1 1] Material Colour
  (bind _returnvalue (`PrimitiveComponent.CreateDynamicMaterialInstance` _mesh 0 (`PrimitiveComponent.GetMaterial` _mesh 0)))
  (bind _newparam (`self.GetRandomColour`))
  (`MaterialInstanceDynamic.SetVectorParameterValue` _returnvalue "BodyColor" _newparam)
  ;;[1 1 1] FX Colours edit
  (bind _asmock_weapon (cast `/Game/Scripts/Blueprints/Weaponry/MockWeapon` (`ChildActorComponent.ChildActor` (`self.MockWeapon`))))
  (`/Game/Scripts/Blueprints/Weaponry/MockWeapon.FXColoursEdit` _asmock_weapon (struct :`R` 0.85 :`B` 0.023408 :`A` 1.0)))

(event `WeaponFire`
  ;[1 1 1] Firing
  (bind _asmock_weapon (cast `/Game/Scripts/Blueprints/Weaponry/MockWeapon` (`ChildActorComponent.ChildActor` (`self.MockWeapon`))))
  (`/Game/Scripts/Blueprints/Weaponry/MockWeapon.WeaponFire` _asmock_weapon))

(fn `GetRandomColour`
  (returns (NewParam :type "LinearColor Structure"))
  (locals (NewLocalVar_0 :type "LinearColor Structure"))
  (bind (_returnvalue_r _returnvalue_g _returnvalue_b _returnvalue_a) (break `LinearColor` (`KismetMathLibrary.HSVToRGB` (`KismetMathLibrary.RandomFloatInRange` 0.0 365.0) (`KismetMathLibrary.RandomFloatInRange` 0.1 1.0) (`KismetMathLibrary.RandomFloatInRange` 0.4 1.0))))
  (return (make `LinearColor` _returnvalue_r _returnvalue_g _returnvalue_b _returnvalue_a)))

(fn `UserConstructionScript`
  (`self.RandomizeAppearance`))