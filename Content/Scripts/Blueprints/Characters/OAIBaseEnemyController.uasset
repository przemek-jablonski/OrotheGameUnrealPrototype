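; AI controller for base enemies that chases the player and fires its weapon.
; BeginPlay randomizes stopping and shooting thresholds, then starts looping timers for movement and shooting.
; Movement calls AIMoveTo targeting the player controller; shooting waits a random delay, then calls FireWeapon on the enemy character.
; The range check compares both pawns' distances from world origin, rather than the distance between them.
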(event `self.ReceiveBeginPlay`
  ;[1 1 1] Begin Play
  (`self.ConstructProperties`)
  (`KismetSystemLibrary.K2_SetTimerDelegate` (delegate `/Game/Scripts/Blueprints/Characters/IAIEnemyController.MoveTowardsTarget`) (`self.AIUpdateTimeSec`) true)
  (`KismetSystemLibrary.K2_SetTimerDelegate` (delegate `/Game/Scripts/Blueprints/Characters/IAIEnemyController.ShootTarget`) (* (`self.AIShootTargetUpdateTimeSec`) (`KismetMathLibrary.RandomFloatInRange` 0.8 1.65)) true))

(event `/Game/Scripts/Blueprints/Characters/IAIEnemyController.ConstructProperties`
  ;[1 1 1] Construct Properties
  (set `self.MoveTowardsPlayerThreshold` (`KismetMathLibrary.RandomFloatInRange` 50.0 350.0))
  (set `self.EnemyShootingDistanceThreshold` (`KismetMathLibrary.RandomFloatInRange` 3000.0 10000.0)))

(event `/Game/Scripts/Blueprints/Characters/IAIEnemyController.MoveTowardsTarget`
  ;[1 1 1] Move Towards Target
  (`|AIMoveTo` (`self.K2_GetPawn`) (0.0 0.0 0.0) (`GameplayStatics.GetPlayerController` 0) (`self.MoveTowardsPlayerThreshold`) true))

(event `/Game/Scripts/Blueprints/Characters/IAIEnemyController.ShootTarget`
  (bind _returnvalue (`self.K2_GetPawn`))
  ;[1 1 1] Shoot Target
  (`KismetSystemLibrary.Delay` (`KismetMathLibrary.RandomFloatInRange` 0.0 (`self.AIShootTargetMaxDelaySec`)))
  (if (<= (`KismetMathLibrary.Abs` (- (`KismetMathLibrary.VSize` (`self.K2_GetActorLocation` (`self.K2_GetPawn` (`GameplayStatics.GetPlayerController` 0)))) (`KismetMathLibrary.VSize` (`self.K2_GetActorLocation` _returnvalue)))) (`self.EnemyShootingDistanceThreshold`))
    (bind _asobase_enemy_character (cast `/Game/Scripts/Blueprints/Characters/OBaseEnemyCharacter` _returnvalue))
    (`/Game/Scripts/Blueprints/Characters/OBaseEnemyCharacter.FireWeapon` _asobase_enemy_character)))

(fn `UserConstructionScript`)