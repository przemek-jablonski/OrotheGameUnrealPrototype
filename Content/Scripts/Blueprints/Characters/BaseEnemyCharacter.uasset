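; Base enemy character Blueprint that provides weapon firing, randomized setup, and damage and death handling.
; FireWeapon triggers the child-actor weapon, while ConstructProperties sets jog speed and a random shooting-distance threshold.
; RandomizeAppearance tints a dynamic mesh material with a random HSV color.
; A damage event subtracts each damage entry from health, prints it, and spawns fire FX before destroying the actor below zero.
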(event `/Game/Scripts/Blueprints/Characters/IEnemy.Spawn`)

(event `/Game/Scripts/Blueprints/Characters/IEnemy.FireWeapon`
  (bind _asomock_weapon_with_projectile (cast `/Game/Scripts/Blueprints/Weaponry/OMockWeaponWithProjectile` (`ChildActorComponent.ChildActor` (`self.Weapon`))))
  (`/Game/Scripts/Blueprints/Weaponry/OMockWeaponWithProjectile.WeaponFire` _asomock_weapon_with_projectile))

(event `/Game/Scripts/Blueprints/Characters/IEnemy.ConstructProperties`
  ;[1 1 1] Starting Movement Speed
  (set `self.CurrentSpeedMultiplier` (`self.JogMultiplier`))
  ;[1 1 1] Shooting Distance
  (set `self.EnemyShootingDistanceThreshold` (+ (`KismetMathLibrary.RandomFloatInRange` 0.0 2000.0) (`self.EnemyShootingDistanceMin`))))

(event `/Game/Scripts/Blueprints/Characters/IEnemy.RandomizeAppearance`
  (bind _mesh (`self.Mesh`))
  ;[1 1 1] Customize Appearance
  ;;[1 1 1] MaterialColour
  (bind _returnvalue (`PrimitiveComponent.CreateDynamicMaterialInstance` _mesh 0 (`PrimitiveComponent.GetMaterial` _mesh 0)))
  (bind _randomcolour (`self.GetRandomColour`))
  (`MaterialInstanceDynamic.SetVectorParameterValue` _returnvalue "BodyColor" _randomcolour))

(event `CustomEvent`
  (params (damageData :type "Array of /Game/Scripts/Blueprints/DataStructures/OSProjectileDamageStruct Structure (by ref)"))
  (bind (_returnvalue_location _returnvalue_rotation _returnvalue_scale) (`KismetMathLibrary.BreakTransform` (`self.GetTransform`)))
  ;[1 1 1] Damaged
  (for _array_element damageData
    (bind _output_get (set `self.CurrentHealthPoints` (- (`self.CurrentHealthPoints`) (`.damageTypeValue_5_E91F56ED41F15A2D7E6080955AB4F4A6` (break `/Game/Scripts/Blueprints/DataStructures/OSProjectileDamageStruct` _array_element)))))
    (`KismetSystemLibrary.PrintString` (`KismetStringLibrary.BuildString_Double` "ENEMY HP: " "" _output_get))
    (if (< _output_get 0.0)
      (`|SpawnActorFromClass` "/Game/Scripts/Blueprints/FXs/FireFX.FireFX_C" (`KismetMathLibrary.MakeTransform` (- _returnvalue_location (0.0 120.0 0.0)) _returnvalue_rotation _returnvalue_scale) "Undefined" "OverrideRootScale")
      (`self.K2_DestroyActor`))))

(fn `GetRandomColour`
  (returns (randomColour :type "LinearColor Structure"))
  (return (`KismetMathLibrary.HSVToRGB` (`KismetMathLibrary.RandomFloatInRange` 0.0 365.0) (`KismetMathLibrary.RandomFloatInRange` 0.6 1.0) (`KismetMathLibrary.RandomFloatInRange` 0.4 1.0))))

(fn `UserConstructionScript`)