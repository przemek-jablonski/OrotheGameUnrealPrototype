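; AI controller for an enemy that pursues the player and fires its weapon, driven by two looping timers.
; Every second it issues a move toward the player controller actor, stopping within a threshold.
; At a randomized interval it calls WeaponFire on EnemyCharacter3 when within a randomized range.
; The range check compares both pawns' distances from world origin, rather than measuring the distance between them.
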(event `self.ReceiveBeginPlay`
  (set `self.EnemyShootingDistanceMin` (+ (`KismetMathLibrary.RandomFloatInRange` 3000.0 10000.0) (`self.MoveTowardPlayerThreshold`)))
  (`KismetSystemLibrary.K2_SetTimerDelegate` (delegate `MoveTowardsPlayer`) 1.0 true)
  (`KismetSystemLibrary.K2_SetTimerDelegate` (delegate `ShootPlayer`) (`KismetMathLibrary.RandomFloatInRange` 0.5 4.0) true))

(event `MoveTowardsPlayer`
  ;[1 1 1] Move Towards Player
  (`|AIMoveTo` (`self.K2_GetPawn`) (0.0 0.0 0.0) (`GameplayStatics.GetPlayerController` 0) (`self.MoveTowardPlayerThreshold`) true))

(event `ShootPlayer`
  ;[1 1 1] Shoot Player
  (if (<= (`KismetMathLibrary.Abs` (- (`KismetMathLibrary.VSize` (`self.K2_GetActorLocation` (`self.K2_GetPawn` (`GameplayStatics.GetPlayerController` 0)))) (`KismetMathLibrary.VSize` (`self.K2_GetActorLocation` (`self.K2_GetPawn`))))) (`self.EnemyShootingDistanceMin`))
    (bind _asenemy_character_3 (cast `/Game/Scripts/Blueprints/Characters/EnemyCharacter3` (`self.K2_GetPawn`)))
    (`/Game/Scripts/Blueprints/Characters/EnemyCharacter3.WeaponFire` _asenemy_character_3)))

(fn `UserConstructionScript`)