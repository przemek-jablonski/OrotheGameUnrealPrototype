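; Player character with camera-relative movement, sprint, spring-arm aim zoom and firing through a mock projectile weapon held as a child actor.
; Vertical look input also rotates the weapon; aiming swaps arm length and socket offset.
; On BeginPlay, a mock assembly spawns a separate weapon body and snaps a grip to its matching Vulcrum attachment point by offsetting root locations.
; DealDamage subtracts each damage entry from health and prints it, without death handling.
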(event `InputAxis|MovementVertical`
  (params (AxisValue :type "Float (single-precision)"))
  (bind (_returnvalue_roll _returnvalue_pitch _returnvalue_yaw) (`KismetMathLibrary.BreakRotator` (`self.GetControlRotation`)))
  ;[1 1 1] Movement
  (`self.AddMovementInput` (`KismetMathLibrary.GetForwardVector` (`KismetMathLibrary.MakeRotator` 0.0 0.0 _returnvalue_yaw)) (* AxisValue (stale `InputAction|Sprint` _output_get))))

(event `InputAxis|MovementHorizontal`
  (params (AxisValue :type "Float (single-precision)"))
  (bind (_returnvalue_roll _returnvalue_pitch _returnvalue_yaw) (`KismetMathLibrary.BreakRotator` (`self.GetControlRotation`)))
  ;[1 1 1] Movement
  (`self.AddMovementInput` (`KismetMathLibrary.GetRightVector` (`KismetMathLibrary.MakeRotator` 0.0 0.0 _returnvalue_yaw)) (* AxisValue (stale `InputAction|Sprint` _output_get))))

(event `InputAction|Sprint`
  (params (Key :type "Key Structure" :default "AnyKey"))
  ;[1 1 1] Movement
  ;;[1 1 1] Sprinting multiplier
  (:`Pressed`
    (set `self.SprintPressed` true)
    (bind _output_get (set `self.CurrentSpeedMultiplier` (`self.SprintMultiplier`))))
  (:`Released`
    (set `self.SprintPressed` false)
    (set `self.CurrentSpeedMultiplier` (`self.JogMultiplier`))))

(event `InputAxis|RotationVertical`
  (params (AxisValue :type "Float (single-precision)"))
  (bind _returnvalue (`GameplayStatics.GetWorldDeltaSeconds`))
  (bind _baseturn (`self.BaseTurn`))
  ;[1 1 1] Rotation
  (`self.AddControllerPitchInput` (* AxisValue _baseturn _returnvalue))
  (`SceneComponent.K2_AddLocalRotation` (`self.Weapon`) (`KismetMathLibrary.MakeRotator` (* AxisValue _returnvalue _baseturn)) false false))

(event `InputAxis|RotationHorizontal`
  (params (AxisValue :type "Float (single-precision)"))
  ;[1 1 1] Rotation
  (`self.AddControllerYawInput` (* (`self.BaseTurn`) (`GameplayStatics.GetWorldDeltaSeconds`) AxisValue)))

(event `CreateWeapon`
  (bind (_returnvalue_location _returnvalue_rotation _returnvalue_scale) (`KismetMathLibrary.BreakTransform` (`self.GetTransform`)))
  (bind _returnvalue (`KismetMathLibrary.MakeTransform` (+ _returnvalue_location (0.0 150.0 0.0)) _returnvalue_rotation _returnvalue_scale))
  ;[1 1 1] Constructing Weapon
  ;;[1 1 1] Spawning BODY
  (bind _returnvalue_2 (`|SpawnActorFromClass` "/Game/Scripts/Blueprints/Weaponry/Parts/OWeaponBodyPart.OWeaponBodyPart_C" _returnvalue "Undefined" "OverrideRootScale"))
  (for _array_element (`self.GetAllChildActors` _returnvalue_2 true)
    (bind _asoweapon_vulcrum_space (cast `/Game/Scripts/Blueprints/Weaponry/Parts/OWeaponVulcrumSpace` _array_element))
    (if (and (`|EnumEquality` (`/Game/Scripts/Blueprints/Weaponry/Parts/OWeaponVulcrumSpace.VulcrumBase` _asoweapon_vulcrum_space) "NewEnumerator0") (`|EnumEquality` (`/Game/Scripts/Blueprints/Weaponry/Parts/OWeaponVulcrumSpace.VulcrumAttachment` _asoweapon_vulcrum_space) "NewEnumerator6"))
      ;;[1 1 1] Spawning GRIP
      (bind _returnvalue_3 (`|SpawnActorFromClass` "/Game/Scripts/Blueprints/Weaponry/Parts/OWeaponGripPart.OWeaponGripPart_C" _returnvalue "Undefined" "OverrideRootScale"))
      (bind _asoweapon_grip_part (cast `/Game/Scripts/Blueprints/Weaponry/Parts/OWeaponGripPart` _returnvalue_3))
      (bind _defaultsceneroot (`/Game/Scripts/Blueprints/Weaponry/Parts/OWeaponBasePart.DefaultSceneRoot` _asoweapon_grip_part))
      (bind _returnvalue_location_2 (`KismetMathLibrary.BreakTransform` (`self.GetTransform` _asoweapon_vulcrum_space)))
      (bind _returnvalue_location_3 (`KismetMathLibrary.BreakTransform` (`SceneComponent.K2_GetComponentToWorld` (`SceneComponent.GetChildComponent` (`/Game/Scripts/Blueprints/Weaponry/Parts/OWeaponGripPart.OWeaponVulcrumSpace` _asoweapon_grip_part) 0))))
      (bind _returnvalue_location_4 (`KismetMathLibrary.BreakTransform` (`SceneComponent.K2_GetComponentToWorld` _defaultsceneroot)))
      (`SceneComponent.K2_SetWorldLocation` _defaultsceneroot (- _returnvalue_location_2 (- _returnvalue_location_3 _returnvalue_location_4)) false true))))

(event `ConstructVariables`
  ;[1 1 1] ConstructVariables
  ;;[1 1 1] Starting Movement Speed
  (set `self.CurrentSpeedMultiplier` (`self.JogMultiplier`))
  ;;[1 1 1] Cam Arm Length (normal)
  (set `self.CamNormalArmLength` (`SpringArmComponent.TargetArmLength` (`self.SpringArm`)))
  (set `SpringArmComponent.TargetArmLength` (`self.CamNormalArmLength`) (`self.SpringArm`))
  ;;[1 1 1] Cam Arm Length (aiming)
  (set `self.CamAimingArmLengthDiv` (/ (`self.CamNormalArmLength`) (`self.CamAimingArmLengthDiv`))))

(event `self.ReceiveBeginPlay`
  ;[1 1 1] Setting variables
  (`self.ConstructVariables`)
  ;[1 1 1] CREATE WEAPON (MOCK)
  (`self.CreateWeapon`))

(event `InputAction|Aim`
  (params (Key :type "Key Structure" :default "AnyKey"))
  (bind _springarm (`self.SpringArm`))
  ;[1 1 1] Aiming
  (:`Pressed`
    (set `SpringArmComponent.TargetArmLength` (`self.CamAimingArmLengthDiv`) _springarm)
    (set `SpringArmComponent.SocketOffset` (`self.CamAimingArmOffset`) _springarm))
  (:`Released`
    (set `SpringArmComponent.TargetArmLength` (`self.CamNormalArmLength`) _springarm)
    (set `SpringArmComponent.SocketOffset` (0.0 0.0 100.0) _springarm)))

(event `InputAction|Fire`
  (params (Key :type "Key Structure" :default "AnyKey"))
  ;[1 1 1] Firing
  (:`Pressed`
    (bind _asomock_weapon_with_projectile (cast `/Game/Scripts/Blueprints/Weaponry/OMockWeaponWithProjectile` (`ChildActorComponent.ChildActor` (`self.Weapon`))))
    (`/Game/Scripts/Blueprints/Weaponry/OMockWeaponWithProjectile.WeaponFire` _asomock_weapon_with_projectile)))

(event `/Game/Scripts/Blueprints/Interfaces/IDamageable.DealDamage`
  (params (damageData :type "Array of /Game/Scripts/Blueprints/DataStructures/OSProjectileDamageStruct Structure (by ref)"))
  ;[1 1 1] Damaged
  (for _array_element damageData
    (bind _output_get (set `self.healthPoints` (- (`self.healthPoints`) (`.damageTypeValue_5_E91F56ED41F15A2D7E6080955AB4F4A6` (break `/Game/Scripts/Blueprints/DataStructures/OSProjectileDamageStruct` _array_element)))))
    (`KismetSystemLibrary.PrintString` (`KismetStringLibrary.BuildString_Double` "PLAYER HP: " "" _output_get))))

(fn `UserConstructionScript`)